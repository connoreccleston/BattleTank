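; AutoMortar is a mortar actor with a turret, a barrel and a health bar widget.
; On BeginPlay it initializes its TankAiming component with the TankBarrel and TankTurret references, then sets up the health bar.
; The health bar setup casts the widget's user object to HealthBar and assigns the mortar as its Tank.
; The graphs hold only this wiring, with no aiming or firing logic.
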(event `self.ReceiveBeginPlay`
  (`TankAimingComponent.Init` (`self.TankAiming`) (`self.TankBarrel`) (`self.TankTurret`))
  (`self.Init Health Bar`))

(fn `Init Health Bar`
  (bind _ashealth_bar (cast `/Game/Blueprints/HealthBar` (`WidgetComponent.GetUserWidgetObject` (`self.Widget`))))
  (set `/Game/Blueprints/HealthBar.Tank` self _ashealth_bar))

(fn `UserConstructionScript`)